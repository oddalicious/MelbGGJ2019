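; Hunt camera actor that follows the player and keeps the player's current target in view.
; On BeginPlay it finds the controlled genericPlayer, copies that pawn's spring arm length and attaches itself, snapped to the pawn's location.
; Each tick, while a target is valid, it aims the spring arm along the player-to-target direction and separately rotates the camera to look at the target.
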(event EventBeginPlay
  (bind _asgeneric_player (Utilities|Casting|CastTogenericPlayer (Pawn|GetControlledPawn (Game|GetPlayerController 0))))
  (bind _output_get (Variables|Default|SetPlayer _asgeneric_player))
  (Variables|/Script/Engine.SpringArmComponent|SetTargetArmLength (Variables|Default|GetSpringArm) (Variables|/Script/Engine.SpringArmComponent|GetTargetArmLength (Variables|/Game/Blueprints/BP_Player.BP_Player_C|GetSpringArm _output_get)))
  (Transformation|AttachActorToActor (Variables|Default|GetPlayer) "None" "SnapToTarget" "KeepRelative" "KeepRelative" true))

(event EventTick
  (params (DeltaSeconds :type Float%20%28single-precision%29))
  (bind _player (Variables|Default|GetPlayer))
  (bind _target (Variables|/Game/Blueprints/genericPlayer.genericPlayer_C|GetTarget _player))
  (Utilities|IsValid _player
    (:Is%20Valid
      (Utilities|IsValid _target
        (:Is%20Valid
          (Variables|Default|SetPlayerTarget (Transformation|GetActorLocation _target))
          (Transformation|SetWorldRotation (Variables|Default|GetSpringArm) (Math|Rotator|FindLookatRotation (Transformation|GetActorLocation _player) (Variables|Default|GetPlayerTarget)) false false)
          (Transformation|SetWorldRotation (Variables|Default|GetCamera) (Utilities|LookatLocation (Variables|Default|GetCamera) (Variables|Default|GetPlayerTarget)) false false))))))

(fn ConstructionScript)