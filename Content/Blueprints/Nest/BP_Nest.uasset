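; BP_Nest is a nest actor where the player delivers rabbits to win the game.
; Its sphere overlap, sized from CollisionSize in the construction script, takes a rabbit from an entering BP_Player through RemoveRabbit.
; Each successful handover increments a count, and reaching WinAmount prints a win message and plays the EndSequence level sequence if one is valid.
; BeginPlay also enables input from the first player controller.
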(event OnComponentBeginOverlap(Sphere)
  (params (OverlappedComponent :type Primitive%20Component%20Object%20Reference) (OtherActor :type Actor%20Object%20Reference) (OtherComp :type Primitive%20Component%20Object%20Reference) (OtherBodyIndex :type Integer) (bFromSweep :type Boolean) (SweepResult :type Hit%20Result%20Structure%20%28by%20ref%29))
  (bind _endsequence (Variables|Default|GetEndSequence))
  (bind _asbp_player (Utilities|Casting|CastToBP_Player OtherActor))
  (bind _valid (Default|RemoveRabbit _asbp_player))
  (if _valid
    (bind _output_get (Variables|Default|SetGivenRabbitCount (+ (Variables|Default|GetGivenRabbitCount) 1)))
    (if (== _output_get (Variables|Default|GetWinAmount))
      ;[0 1 0.09881] Win the game
      (Development|PrintString "You are Winnar")
      (Utilities|IsValid _endsequence
        (:Is%20Valid
          (bind _returnvalue (Sequencer|Player|CreateLevelSequencePlayer _endsequence))
          (Sequencer|Player|Play _returnvalue :!class /Script/MovieScene.MovieSceneSequencePlayer))))))

(event EventBeginPlay
  (Input|EnableInput (Game|GetPlayerController 0)))

(fn ConstructionScript
  (Components|Sphere|SetSphereRadius (Variables|Default|GetSphere) (Variables|Default|GetCollisionSize) true))