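; Player eagle pawn that flies constantly forward, steered by pitch and yaw input, with flap, dive and hunt abilities.
; Tick moves it along its arrow and eases speed by pitch, while movement and action state enums gate inputs.
; Timelines drive flap boosts, dives with camera lag, blur and shake, and out-of-bounds turn-backs.
; A speed-scaled downward trace pulls it off the ground; hunting blends to a separate camera, and death only prints.
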(event OnComponentBeginOverlap(Body)
  (params (OverlappedComponent :type Primitive%20Component%20Object%20Reference) (OtherActor :type Actor%20Object%20Reference) (OtherComp :type Primitive%20Component%20Object%20Reference) (OtherBodyIndex :type Integer) (bFromSweep :type Boolean) (SweepResult :type Hit%20Result%20Structure%20%28by%20ref%29))
  ;[1 1 1] Ground Collision (Death)
  (if (== (Utilities|GetClass OtherActor) "/Script/Landscape.Landscape")
    (Utilities|FlowControl|DoOnce false
      (:Completed
        (Development|PrintString "should die")))))

(event Custom|PlayDive
  ;[1 1 1] Diving
  (Variables|Movement|SetYawAxis 0.0)
  (Timeline|DiveTimeline PlayFromStart
    (:Update
      (Diving|DiveTick))
    (:Finished
      (if (Utilities|Enum|Equal(Enum) (Variables|Default|GetPlayerActionState) "NewEnumerator1")
        (CallFunction|PlayDive)
        (else
          (CallFunction|PlayCameraReset)
          (Utilities|FlowControl|Delay (Variables|Dive|GetDiveCoolDown))
          (CallFunction|ResetDive))))))

(event Custom|PlayCameraReset
  (bind _resetdivecameratimeline (Variables|Default|GetResetDiveCameraTimeline))
  (bind _returnvalue (Components|Timeline|GetPlaybackPosition _resetdivecameratimeline))
  ;[1 1 1] Diving
  (Timeline|ResetDiveCameraTimeline PlayFromStart
    (:Update
      (Diving|ResetDiveCamera _returnvalue)
      (Rendering|Material|SetScalarParameterValue "/Game/Effects/MPC_PostProcessorss.MPC_PostProcessorss" "Blur" (Math|Float|Lerp 1.0 0.0 _returnvalue) :!class /Script/Engine.KismetMaterialLibrary))
    (:Finished
      (Variables|/Script/Engine.SpringArmComponent|SetCameraLagSpeed (Variables|Default|GetSpringArm) 0.0))))

(event Custom|OutOfBounds
  (params (Direction :type Rotator) (Angle :type Float%20%28single-precision%29))
  ;[1 1 1] Out of Bounds
  (if (Utilities|Enum|NotEqual(Enum) (Variables|Default|GetPlayerMovementState) "NewEnumerator10")
    (OutOfBounds|SetUpOutOfBounds Angle)
    (Timeline|GoBackInTimeline PlayFromStart
      (:Update
        (OutOfBounds|OutOfBoundsTick Direction))
      (:Finished
        (Variables|OutOfBounds|SetBoundCollisionAngle 0.0)
        (Utilities|FlowControl|Delay (Variables|OutOfBounds|GetOutOfBoundsCoolDown))
        (Variables|Default|SetPlayerMovementState "NewEnumerator8")
        (Variables|Default|SetPlayerActionState "NewEnumerator3")))))

(event Custom|PlayFlap
  ;[1 1 1] Flapping
  (if (Utilities|Enum|Equal(Enum) (Variables|Default|GetPlayerActionState) "NewEnumerator0")
    (Flapping|SetUpFlap)
    (|FlapAnimationTrigger)
    (Timeline|FlapTimeline PlayFromStart
      (:Update
        (Flapping|FlapTick))
      (:Finished
        (Utilities|FlowControl|Delay (Variables|Flapping|GetFlapHoldCoolDown))
        (CallFunction|PlayFlap)))))

(event Custom|ResetDive
  ;[1 1 1] Diving
  (Utilities|FlowControl|DoOnce false) ; enters at Reset
)

(event Custom|PlayDiveCameraSet
  (bind _setdivecameratimeline (Variables|Default|GetSetDiveCameraTimeline))
  (bind _returnvalue (Components|Timeline|GetPlaybackPosition _setdivecameratimeline))
  ;[1 1 1] Diving
  (Timeline|SetDiveCameraTimeline PlayFromStart
    (:Update
      (Diving|SetDiveCamera _returnvalue)
      (Rendering|Material|SetScalarParameterValue "/Game/Effects/MPC_PostProcessorss.MPC_PostProcessorss" "Blur" _returnvalue :!class /Script/Engine.KismetMaterialLibrary))))

(event EventTick
  (params (DeltaSeconds :type Float%20%28single-precision%29))
  (bind _arrow (Variables|Default|GetArrow))
  (bind _sm_eagle (Variables|Default|GetSM_Eagle))
  (bind _returnvalue (Math|Vector|GetForwardVector _arrow))
  (bind _returnvalue_2 (Transformation|GetRelativeTransform _sm_eagle))
  (bind _returnvalue_3 (Math|Transform|InverseTransformDirection _returnvalue_2 _returnvalue))
  ;[1 1 1] Tick - Speed Manager
  (Transformation|AddActorLocalOffset (* (Math|Vector|MakeVector (.x _returnvalue_3) (.y _returnvalue_3) (.z _returnvalue_3)) (* (Utilities|Time|GetWorldDeltaSeconds) (Variables|Speed|GetSpeed))) true false)
  (Locomotion|DirectionSpeed)
  (OutOfBounds|ShootTrace)
  (Locomotion|ResetRoll))

(event EventBeginPlay
  ;[1 1 1] Begin Play
  (StartUp|SetupTimelines)
  (StartUp|GetHuntCamera))

(event Input|ActionEvents|InputActionDive
  (params (Key :type Key%20Structure))
  ;[1 1 1] Diving
  (:Pressed
    (Utilities|FlowControl|DoOnce false
      (:Completed
        (switch Utilities|FlowControl|Switch|SwitchonEPlayerActionStates (Variables|Default|GetPlayerActionState)
          (:NewEnumerator3
            _)
          (:NewEnumerator0
            _)
          (:NewEnumerator2
            _))
        (Variables|Default|SetPlayerActionState "NewEnumerator1")
        (CallFunction|PlayDive)
        (CallFunction|PlayDiveCameraSet))))
  (:Released
    (Variables|Default|SetPlayerActionState "NewEnumerator3")
    (Variables|Default|SetPlayerMovementState "NewEnumerator8")))

(event Input|ActionEvents|InputActionFlap
  (params (Key :type Key%20Structure))
  ;[1 1 1] Flapping
  (:Pressed
    (switch Utilities|FlowControl|Switch|SwitchonEPlayerActionStates (Variables|Default|GetPlayerActionState)
      (:NewEnumerator3
        (Variables|Default|SetPlayerActionState "NewEnumerator0")
        (CallFunction|PlayFlap))))
  (:Released
    (Audio|Components|Audio|Stop (Variables|Default|GetFlapTimeline))
    (Utilities|FlowControl|Delay (Variables|Flapping|GetFlapEndCoolDown))
    (Variables|Default|SetPlayerMovementState "NewEnumerator8")
    (Variables|Default|SetPlayerActionState "NewEnumerator3")))

(event Input|ActionEvents|InputActionPause
  (params (Key :type Key%20Structure))
  ;[1 1 1] PauseGame
  (:Pressed
    (bind _asbp_game_jam_kit_in_game_hud (Utilities|Casting|CastToBP_GameJamKit_InGame_HUD (HUD|GetHUD (Game|GetPlayerController 0))))
    (Default|SetPaused _asbp_game_jam_kit_in_game_hud true)))

(event Input|ActionEvents|InputActionHunt
  (params (Key :type Key%20Structure))
  ;[1 1 1] Hunting
  (:Released
    (Hunting|EndHunt)))

(event Input|AxisEvents|InputAxisPitch
  (params (AxisValue :type Float%20%28single-precision%29))
  ;[1 1 1] Pitch
  (bind _oaxis (Utilities|AxisHandler AxisValue)
    (:then
      (switch Utilities|FlowControl|Switch|SwitchonEPlayerMovementStates (Variables|Default|GetPlayerMovementState)
        (:NewEnumerator0
          _)
        (:NewEnumerator2
          _)
        (:NewEnumerator3
          _)
        (:NewEnumerator8
          _))
      (Locomotion|PitchRotation _oaxis))
    (:Zero
      (switch Utilities|FlowControl|Switch|SwitchonEPlayerMovementStates (Variables|Default|GetPlayerMovementState)
        (:NewEnumerator2
          _)
        (:NewEnumerator3
          _)
        (:NewEnumerator8
          _))
      (Variables|Default|SetPlayerMovementState "NewEnumerator8")
      (Locomotion|ResetPitch))))

(event Input|AxisEvents|InputAxisYaw
  (params (AxisValue :type Float%20%28single-precision%29))
  ;[1 1 1] Turning
  (bind _oaxis (Utilities|AxisHandler AxisValue)
    (:then
      (switch Utilities|FlowControl|Switch|SwitchonEPlayerMovementStates (Variables|Default|GetPlayerMovementState)
        (:NewEnumerator0
          (Locomotion|TurnRotation _oaxis :!label _label))
        (:NewEnumerator2
          _)
        (:NewEnumerator3
          _)
        (:NewEnumerator4
          (goto _label))
        (:NewEnumerator5
          (goto _label))
        (:NewEnumerator8
          (goto _label))))
    (:Zero
      (switch Utilities|FlowControl|Switch|SwitchonEPlayerMovementStates (Variables|Default|GetPlayerMovementState)
        (:NewEnumerator0
          _)
        (:NewEnumerator2
          _)
        (:NewEnumerator3
          _)
        (:NewEnumerator4
          (Variables|Default|SetPlayerMovementState "NewEnumerator8" :!label _label_2))
        (:NewEnumerator5
          (goto _label_2))
        (:NewEnumerator8
          (goto _label_2)))))
  (Locomotion|SetTurnAnimationAxis _oaxis))

(fn ConstructionScript
  (Variables|/Script/Engine.SpringArmComponent|SetCameraRotationLagSpeed (Variables|Default|GetSpringArm) (Variables|Default|GetDefaultCameraLag))
  (Variables|Speed|SetSpeed (Variables|Speed|GetDefaultSpeed)))

(fn ResetPitch
  (bind _returnvalue (Utilities|Time|GetWorldDeltaSeconds))
  (bind _resetspeed (Variables|ResetOrientation|GetResetSpeed))
  (bind _easetype (Variables|ResetOrientation|GetEaseType))
  (bind _blendexp (Variables|ResetOrientation|GetBlendExp))
  (bind _steps (Variables|ResetOrientation|GetSteps))
  (bind _sm_eagle (Variables|Default|GetSM_Eagle))
  (bind _returnvalue_2 (* _returnvalue _resetspeed))
  (bind _relativerotation (Variables|/Script/Engine.SceneComponent|GetRelativeRotation _sm_eagle))
  (bind _result (Math|Interpolation|Ease _easetype _returnvalue_2 (.pitch _relativerotation) 0.0 _blendexp _steps))
  (Transformation|SetRelativeRotation (Variables|Default|GetSM_Eagle) (Math|Rotator|MakeRotator (.roll _relativerotation) _result (.yaw _relativerotation)) false false)
  (if (< _result 0.0)
    (if (> _result -4.0)
      (Variables|Default|SetPlayerMovementState "NewEnumerator0" :!label _label))
    (elif (< _result 4.0)
      (goto _label))))

(fn ResetRoll
  (bind _returnvalue (Utilities|Time|GetWorldDeltaSeconds))
  (bind _steps (Variables|ResetOrientation|GetSteps))
  (bind _resetspeed (Variables|ResetOrientation|GetResetSpeed))
  (bind _easetype (Variables|ResetOrientation|GetEaseType))
  (bind _blendexp (Variables|ResetOrientation|GetBlendExp))
  (bind _sm_eagle (Variables|Default|GetSM_Eagle))
  (bind _returnvalue_2 (* _returnvalue _resetspeed))
  (bind _relativerotation (Variables|/Script/Engine.SceneComponent|GetRelativeRotation _sm_eagle))
  (bind _result (Math|Interpolation|Ease _easetype _returnvalue_2 (.roll _relativerotation) 0.0 _blendexp _steps))
  (Transformation|SetRelativeRotation (Variables|Default|GetSM_Eagle) (Math|Rotator|MakeRotator (Math|Float|SelectFloat 0.0 _result (< _result 0.01)) (.pitch _relativerotation) (.yaw _relativerotation)) false false))

(fn RotatetoDive
  (params (Alpha :type Float%20%28single-precision%29))
  (bind _sm_eagle (Variables|Default|GetSM_Eagle))
  (bind _relativerotation (Variables|/Script/Engine.SceneComponent|GetRelativeRotation _sm_eagle))
  (bind (_roll _pitch _yaw) (Math|Rotator|BreakRotator _relativerotation))
  (Transformation|SetRelativeRotation (Variables|Default|GetSM_Eagle) (Math|Rotator|SelectRotator "0, 0, 0" (Math|Rotator|MakeRotator _roll (Math|Float|Lerp _pitch (Variables|Dive|GetDivePitch) Alpha) _yaw) (Variables|Hunting|GetbHunting)) false false))

(fn DirectionSpeed
  (if (< (.pitch (Transformation|GetWorldRotation (Variables|Default|GetArrow))) (* (Variables|Speed|GetTurnAngle) -1.0))
    (Variables|Speed|SetSpeed (Math|Float|Lerp (Variables|Speed|GetSpeed) (Variables|Speed|GetDownSpeed) (* (Utilities|Time|GetWorldDeltaSeconds) (Variables|Speed|LerpSpeed|GetDownRate))))
    (elif (> (.pitch (Transformation|GetWorldRotation (Variables|Default|GetArrow))) (Variables|Speed|GetTurnAngle))
      (Variables|Speed|SetSpeed (Math|Float|Lerp (Variables|Speed|GetSpeed) (Variables|Speed|GetUpSpeed) (* (Utilities|Time|GetWorldDeltaSeconds) (Variables|Speed|LerpSpeed|GetUpRate))))
      (else
        (Variables|Speed|SetSpeed (Math|Float|Lerp (Variables|Speed|GetSpeed) (Variables|Speed|GetDefaultSpeed) (* (Utilities|Time|GetWorldDeltaSeconds) (Variables|Speed|LerpSpeed|GetDefaultRate))))))))

(fn SetDiveCamera
  (params (Alpha :type Float%20%28single-precision%29))
  (bind _springarm (Variables|Default|GetSpringArm))
  (bind _divecameralag (Variables|Dive|GetDiveCameraLag))
  (Variables|/Script/Engine.SpringArmComponent|SetCameraRotationLagSpeed _springarm (Math|Float|Lerp (Variables|Default|GetDefaultCameraLag) _divecameralag Alpha))
  (Variables|/Script/Engine.SpringArmComponent|SetCameraLagSpeed _springarm (Math|Float|Lerp 1e+03 (* _divecameralag 1.0) Alpha)))

(fn ResetDiveCamera
  (params (Alpha :type Float%20%28single-precision%29))
  (bind _divecameralag (Variables|Dive|GetDiveCameraLag))
  (bind _springarm (Variables|Default|GetSpringArm))
  (Variables|/Script/Engine.SpringArmComponent|SetCameraRotationLagSpeed _springarm (Math|Float|Lerp _divecameralag (Variables|Default|GetDefaultCameraLag) Alpha))
  (Variables|/Script/Engine.SpringArmComponent|SetCameraLagSpeed _springarm (Math|Float|Lerp _divecameralag 1e+02 Alpha)))

(fn SetupTimelines
  (Utilities|SetupLerpTimeline (Variables|Default|GetDiveTimeline) "/Game/Data/Curve_LinearLerp_Float.Curve_LinearLerp_Float" (Variables|Dive|GetDaveRate) 1.0 false
    (:__
      (Utilities|SetupLerpTimeline (Variables|Default|GetFlapTimeline) "/Game/Data/Curve_LinearLerp_Float.Curve_LinearLerp_Float" (Variables|Flapping|GetFlapRate) 1.0 false
        (:__
          (Utilities|SetupLerpTimeline (Variables|Default|GetResetDiveCameraTimeline) "/Game/Data/Curve_LinearLerp_Float.Curve_LinearLerp_Float" (Variables|Dive|GetCameraResetSpeed) 1.0 false
            (:__
              (Utilities|SetupLerpTimeline (Variables|Default|GetGoBackInTimeline) "/Game/Data/Curve_LinearLerp_Float.Curve_LinearLerp_Float" (Variables|OutOfBounds|GetGoBackRate) 1.0 false
                (:__
                  (Utilities|SetupLerpTimeline (Variables|Default|GetSetDiveCameraTimeline) "/Game/Data/Curve_LinearLerp_Float.Curve_LinearLerp_Float" (Variables|Dive|GetDiveEffectSpeed) 1.0 false))))))))))

(fn TempHuntTick
  (if (Variables|Hunting|GetbHunting)
    (Hunting|HuntTick)
    (bind _output_get (Variables|Hunting|SetStamina (Math|Float|Max(Float) (- (Variables|Hunting|GetStamina) (* (Variables|Hunting|GetStamina) 0.0)) 0.0)))
    (if (== _output_get 0.0)
      _)))

(fn HuntTick
  (bind _target (Variables|Hunting|GetTarget))
  (if (and (Utilities|IsValid _target) (not (Variables|/Game/Blueprints/GrabTarget/Generic/BP_GrabActor.BP_GrabActor_C|GetGrabbed _target)))
    (Transformation|SetWorldRotation (Variables|/Game/Blueprints/huntCamera.huntCamera_C|GetSpringArm (Variables|Hunting|GetHuntCamera)) (Math|Rotator|FindLookatRotation (Transformation|GetActorLocation) (Transformation|GetActorLocation _target)) false false)
    (else
      (Hunting|EndHunt))))

(fn EndHunt
  (Utilities|IsValid (Variables|Hunting|GetTarget)
    (:Is%20Valid
      (Default|EndTarget (Variables|Hunting|GetTarget)))
    (:Is%20Not%20Valid
      _))
  (Variables|Hunting|SetTarget 0)
  (Variables|Hunting|SetbHunting false)
  (Game|Player|SetViewTargetwithBlend (Game|GetPlayerController 0) self 0.5 "VTBlend_Linear" 0.0 false))

(fn BeginHunt
  (params (inTarget :type BP%20Grab%20Actor%20Object%20Reference))
  (Variables|Hunting|SetbHunting true)
  (Variables|Hunting|SetTarget inTarget)
  (Game|Player|SetViewTargetwithBlend (Game|GetPlayerController 0) (Variables|Hunting|GetHuntCamera) 0.5 "VTBlend_Linear" 0.0 false))

(fn PitchRotation
  (params (PitchAxis :type Float%20%28single-precision%29))
  (bind _sm_eagle (Variables|Default|GetSM_Eagle))
  (bind _relativerotation (Variables|/Script/Engine.SceneComponent|GetRelativeRotation _sm_eagle))
  (if (Utilities|Enum|NotEqual(Enum) (Variables|Default|GetPlayerActionState) "NewEnumerator1")
    (if (not (== PitchAxis 0.0))
      (if (> PitchAxis 0.0)
        (Variables|Default|SetPlayerMovementState "NewEnumerator2")
        (else
          (Variables|Default|SetPlayerMovementState "NewEnumerator3")))
      (Transformation|AddLocalRotation (Variables|Default|GetSM_Eagle) (Math|Rotator|MakeRotator 0.0 (Utilities|RotationLerp (* (Utilities|Time|GetWorldDeltaSeconds) (Variables|Movement|GetPitchRate)) PitchAxis) 0.0) false false)
      (Transformation|SetRelativeRotation _sm_eagle (Math|Rotator|MakeRotator (.roll _relativerotation) (Math|Float|Clamp(Float) (.pitch _relativerotation) -6e+01 6e+01) (.yaw _relativerotation)) false false))))

(fn GetHuntCamera
  (bind _outactors (Actor|GetAllActorsOfClass "/Game/Blueprints/huntCamera.huntCamera_C"))
  (Variables|Hunting|SetHuntCamera (Utilities|Array|Get(acopy) _outactors)))

(fn SetTurnAnimationAxis
  (params (Axis :type Float%20%28single-precision%29))
  (bind _output_get (Variables|Movement|SetYawAxis (Math|Float|Lerp (Variables|Movement|GetYawAxis) (Math|Float|SelectFloat 0.0 Axis (or (Variables|Dive|GetbDiving) (Variables|Movement|GetbPitching))) (* (Utilities|Time|GetWorldDeltaSeconds) (Variables|Movement|GetYawSpeed))))))

(fn TurnRotation
  (params (Axis :type Float%20%28single-precision%29))
  (if (Utilities|Enum|NotEqual(Enum) (Variables|Default|GetPlayerActionState) "NewEnumerator1")
    (if (not (== Axis 0.0))
      (if (> Axis 0.0)
        (Variables|Default|SetPlayerMovementState "NewEnumerator5")
        (else
          (Variables|Default|SetPlayerMovementState "NewEnumerator4")))
      (Transformation|AddLocalRotation (Variables|Default|GetSM_Eagle) (Math|Rotator|MakeRotator 0.0 0.0 (Utilities|RotationLerp (* (Utilities|Time|GetWorldDeltaSeconds) (Variables|Movement|GetYawRate)) Axis)) false false))))

(fn FlapDirection
  (if (Utilities|Enum|Equal(Enum) (Variables|Default|GetPlayerMovementState) "NewEnumerator4")
    (Transformation|AddLocalRotation (Variables|Default|GetSM_Eagle) (Math|Rotator|MakeRotator 0.0 0.0 (Utilities|RotationLerp (* (Utilities|Time|GetWorldDeltaSeconds) (Variables|Movement|GetYawRate)) -1.0)) false false)
    (elif (Utilities|Enum|Equal(Enum) (Variables|Default|GetPlayerMovementState) "NewEnumerator5")
      (Transformation|AddLocalRotation (Variables|Default|GetSM_Eagle) (Math|Rotator|MakeRotator 0.0 0.0 (Utilities|RotationLerp (* (Utilities|Time|GetWorldDeltaSeconds) (Variables|Movement|GetYawRate)) 1.0)) false false)
      (else
        (Transformation|AddLocalRotation (Variables|Default|GetSM_Eagle) (Math|Rotator|MakeRotator 0.0 (Utilities|RotationLerp (* (Utilities|Time|GetWorldDeltaSeconds) (Variables|Movement|GetPitchRate)) 1.0) 0.0) false false)))))

(fn FlapTick
  (Variables|Speed|SetSpeed (Math|Float|Clamp(Float) (Math|Float|Lerp (Variables|Flapping|GetPrevSpeed) (Variables|Flapping|GetFlapSpeed) (Components|Timeline|GetPlaybackPosition (Variables|Default|GetFlapTimeline))) 0.0 (Variables|Speed|GetMaxSpeed)))
  (Flapping|FlapDirection))

(fn DiveTick
  (bind _divetimeline (Variables|Default|GetDiveTimeline))
  (bind _returnvalue (Components|Timeline|GetPlaybackPosition _divetimeline))
  (Variables|Speed|SetSpeed (Math|Float|Lerp (Variables|Speed|GetSpeed) (Variables|Dive|GetDiveSpeed) _returnvalue))
  (Diving|RotatetoDive _returnvalue)
  (Class|PlayerController|ClientPlayCameraShake (Game|GetPlayerController 0) "/Game/Effects/BP_CameraShake.BP_CameraShake_C" 1.0 "CameraLocal" "0, 0, 0"))

(fn SetUpFlap
  (Variables|Default|SetPlayerMovementState "NewEnumerator8")
  (bind _output_get (Variables|Flapping|SetPrevSpeed (Variables|Speed|GetSpeed)))
  (Variables|Flapping|SetFlapSpeed (+ _output_get (Variables|Flapping|GetFlapAdd))))

(fn SetUpOutOfBounds
  (params (Angle :type Float%20%28single-precision%29))
  (Variables|OutOfBounds|SetBoundsRotation (Transformation|GetWorldRotation (Variables|Default|GetSM_Eagle)))
  (Variables|OutOfBounds|SetBoundCollisionAngle Angle)
  (Variables|Default|SetPlayerMovementState "NewEnumerator10")
  (Variables|Default|SetPlayerActionState "NewEnumerator4")
  (return))

(fn OutOfBoundsTick
  (params (TargetRotation :type Rotator))
  (Transformation|SetWorldRotation (Variables|Default|GetSM_Eagle) (Math|Rotator|Lerp(Rotator) (Variables|OutOfBounds|GetBoundsRotation) TargetRotation (Components|Timeline|GetPlaybackPosition (Variables|Default|GetGoBackInTimeline)) true) false false))

(fn SetStaminaSaturation
  (params (Alpha :type Float%20%28single-precision%29))
  (Variables|/Script/Engine.CameraComponent|SetPostProcessSettings (Variables|Default|GetCamera) (Utilities|Struct|MakePostProcessSettings (Math|Vector4|MakeVector4 (Math|Float|Lerp 1.0 0.0 Alpha) (Math|Float|Lerp 1.0 0.0 Alpha) (Math|Float|Lerp 1.0 0.0 Alpha) 1.0))))

(fn ShootTrace
  (bind _returnvalue (Transformation|GetActorLocation))
  (bind (_x _y _z) (Math|Vector|BreakVector _returnvalue))
  (bind _returnvalue_2 (Collision|LineTraceByChannel _returnvalue (Math|Vector|MakeVector _x _y (- _z (/ (Variables|Speed|GetSpeed) 2.0))) "TraceTypeQuery1" true 0 "None"))
  (if _returnvalue_2
    (if (Utilities|Enum|Equal(Enum) (Variables|Default|GetPlayerActionState) "NewEnumerator1")
      (Audio|Components|Audio|Stop (Variables|Default|GetDiveTimeline))
      (CallFunction|ResetDive)
      (CallFunction|PlayCameraReset))
    (Variables|Default|SetPlayerMovementState "NewEnumerator10")
    (Variables|Default|SetPlayerActionState "NewEnumerator4")
    (Transformation|AddLocalRotation (Variables|Default|GetSM_Eagle) (Math|Rotator|MakeRotator 0.0 (Utilities|RotationLerp (* (Utilities|Time|GetWorldDeltaSeconds) (Variables|OutOfBounds|GetUpAngle)) 1.0) 0.0) false false)
    (Variables|OutOfBounds|SetbHitGround true)
    (elif (Variables|OutOfBounds|GetbHitGround)
      (Variables|OutOfBounds|SetbHitGround false)
      (Variables|Default|SetPlayerMovementState "NewEnumerator8")
      (Variables|Default|SetPlayerActionState "NewEnumerator3"))))