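; Player Blueprint with a hunt mode that switches to a level-placed HuntCamera to track a target.
; BeginHunt and EndHunt blend the view between camera and player; releasing Screwaround also ends the hunt.
; While hunting, Tick drains Stamina proportionally, with no action at zero, and HuntTick aims the camera's spring arm from player toward target.
; Hunts end when the target is invalid, grabbed or closer than MaxHuntLength.
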(event EventTick
  (params (DeltaSeconds :type Float%20%28single-precision%29))
  (|CallParentFunction DeltaSeconds)
  (if (Variables|Default|Gethunting)
    (CallFunction|HuntTick)
    (bind _output_get (Variables|Default|SetStamina (Math|Float|Max(Float) (- (Variables|Default|GetStamina) (* (Variables|Default|GetStamina) DeltaSeconds)) 0.0)))
    (if (== _output_get 0.0)
      _)))

(event EventBeginPlay
  (|CallParentFunction)
  (bind _outactors (Actor|GetAllActorsOfClass "/Game/Blueprints/huntCamera.huntCamera_C"))
  (Variables|Default|SethuntCamera (Utilities|Array|Get(acopy) _outactors)))

(event Input|ActionEvents|InputActionScrewaround
  (params (Key :type Key%20Structure))
  (:Released
    (CallFunction|EndHunt)))

(fn ConstructionScript)

(fn BeginHunt
  (params (inTarget :type BP%20Grab%20Actor%20Object%20Reference))
  (Variables|Default|Sethunting true)
  (Variables|Default|SetTarget inTarget)
  (Game|Player|SetViewTargetwithBlend (Game|GetPlayerController 0) (Variables|Default|GethuntCamera) 0.5 "VTBlend_Linear" 0.0 false))

(fn EndHunt
  (Variables|Default|SetTarget 0)
  (Variables|Default|Sethunting false)
  (Game|Player|SetViewTargetwithBlend (Game|GetPlayerController 0) self 0.5 "VTBlend_Linear" 0.0 false))

(fn HuntTick
  (bind _returnvalue (Transformation|GetActorLocation))
  (bind _target (Variables|Default|GetTarget))
  (bind _returnvalue_2 (Transformation|GetActorLocation _target))
  (if (Math|Boolean|ANDBoolean (Utilities|IsValid _target) (not (Variables|/Game/Blueprints/GrabTarget/Generic/BP_GrabActor.BP_GrabActor_C|GetGrabbed _target)) (>= (Math|Vector|VectorLength (- _returnvalue_2 _returnvalue)) (Variables|Default|GetMaxHuntLength)))
    (Transformation|SetWorldRotation (Variables|/Game/Blueprints/huntCamera.huntCamera_C|GetSpringArm (Variables|Default|GethuntCamera)) (Math|Rotator|FindLookatRotation _returnvalue _returnvalue_2) false false)
    (else
      (CallFunction|EndHunt))))