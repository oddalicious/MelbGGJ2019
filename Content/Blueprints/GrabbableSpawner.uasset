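; Spawner actor that populates the area around itself with BP_RabbitTarget actors and registers each with the level's TargetManager.
; On BeginPlay it caches the first TargetManager found and starts a looping timer that calls SpawnRabbits until MaxNumRabbits is reached.
; Each spawn lands slightly above a random navigable point within Radius, which the construction script also applies to the Sphere component.
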(event EventBeginPlay
  (bind _outactors (Actor|GetAllActorsOfClass "/Game/Blueprints/TargetManager.TargetManager_C"))
  (Variables|Default|SetTargetmanagerRef (Utilities|Array|Get(acopy) _outactors))
  (Utilities|Time|SetTimerbyFunctionName 0 "SpawnRabbits" 0.5 true))

(fn ConstructionScript
  (Components|Sphere|SetSphereRadius (Variables|Default|GetSphere) (Variables|Default|GetRadius) false))

(fn SpawnRabbits
  (Class|KismetMathLibrary|SeedRandomStream (LocalVariables|Getstream))
  (bind _returnvalue (Game|SpawnActorfromClass "/Game/Blueprints/GrabTarget/Animal/BP_RabbitTarget.BP_RabbitTarget_C" (Math|Transform|MakeTransform (+ (.RandomLocation (Class|NavigationSystemV1|GetRandomPointinNavigableRadius (Transformation|GetActorLocation) (Variables|Default|GetRadius) 0 0)) "0, 0,100.000000")) "Undefined" 0 0))
  (Default|AddTarget (Variables|Default|GetTargetmanagerRef) _returnvalue)
  (bind _output_get (Variables|Default|SetSpawnedRabbitCount (+ (Variables|Default|GetSpawnedRabbitCount) 1)))
  (if (>= _output_get (Variables|Default|GetMaxNumRabbits))
    (Utilities|Time|ClearTimerbyFunctionName 0 "SpawnRabbits")))