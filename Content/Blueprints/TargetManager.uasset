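; TargetManager is an actor that finds grab targets for the player's hunt action.
; On BeginPlay it enables input and caches every BP_GrabActor in the level.
; When Screwaround is pressed, it picks the nearest valid cached actor within the game mode's HuntRange, using each actor's DistPlayer.
; It passes any result to the controlled genericPlayer pawn via BeginHunt.
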(event EventBeginPlay
  (Input|EnableInput (Game|GetPlayerController 0))
  (bind _outactors (Actor|GetAllActorsOfClass "/Game/Blueprints/GrabTarget/Generic/BP_GrabActor.BP_GrabActor_C"))
  (Variables|Default|SetgrabActors _outactors))

(event Collision|EventActorBeginOverlap
  (params (OtherActor :type Actor%20Object%20Reference)))

(event EventTick
  (params (DeltaSeconds :type Float%20%28single-precision%29)))

(event Input|ActionEvents|InputActionScrewaround
  (params (Key :type Key%20Structure))
  (:Pressed
    (bind _outtarget (CallFunction|FindNearestGrabWithinRange))
    (Utilities|IsValid _outtarget
      (:Is%20Valid
        (bind _asgeneric_player (Utilities|Casting|CastTogenericPlayer (Pawn|GetControlledPawn (Game|GetPlayerController 0))))
        (Default|BeginHunt _asgeneric_player _outtarget)))))

(fn ConstructionScript)

(fn FindNearestGrabWithinRange
  (bind _asbp_temp_game_mode (Utilities|Casting|CastToBP_TempGameMode (Game|GetGameMode)))
  (LocalVariables|SetlowestRange (Variables|/Game/Blueprints/BP_TempGameMode.BP_TempGameMode_C|GethuntRange _asbp_temp_game_mode))
  (for _array_element (Variables|Default|GetgrabActors)
    (Utilities|IsValid _array_element
      (:Is%20Valid
        (bind _distance (Default|DistPlayer _array_element))
        (if (< _distance (LocalVariables|GetlowestRange))
          (LocalVariables|Settarget _array_element)
          (LocalVariables|SetlowestRange _distance)))))
  (return (LocalVariables|Gettarget)))