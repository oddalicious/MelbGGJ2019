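; Grabbable target actor that slows time as the player approaches and offers a look-at camera.
; Overlapping SloMoSphere starts slow motion and GrabSphere restores time, both driving global time dilation through timelines.
; Holding Screwaround blends the view to this actor, its spring arm sized and aimed from the player's position each Tick.
; StickToClaws attaches it to PlayerRef's Claw socket but is not called here; debug prints remain.
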(event OnComponentBeginOverlap(grabSphere)
  (params (OverlappedComponent :type Primitive%20Component%20Object%20Reference) (OtherActor :type Actor%20Object%20Reference) (OtherComp :type Primitive%20Component%20Object%20Reference) (OtherBodyIndex :type Integer) (bFromSweep :type Boolean) (SweepResult :type Hit%20Result%20Structure%20%28by%20ref%29))
  (Utilities|Casting|CastTogenericPlayer OtherActor)
  (CallFunction|BeginGrabSequence)
  (bind _newtrack_0 (Timeline|TLExitSlowMo PlayFromStart)
    (:Update
      (Utilities|Time|SetGlobalTimeDilation _newtrack_0))))

(event OnComponentBeginOverlap(SloMoSphere)
  (params (OverlappedComponent :type Primitive%20Component%20Object%20Reference) (OtherActor :type Actor%20Object%20Reference) (OtherComp :type Primitive%20Component%20Object%20Reference) (OtherBodyIndex :type Integer) (bFromSweep :type Boolean) (SweepResult :type Hit%20Result%20Structure%20%28by%20ref%29))
  (Utilities|Casting|CastTogenericPlayer OtherActor)
  (CallFunction|BeginSlowMo)
  (bind _newtrack_0 (Timeline|TLEnterSlowMo PlayFromStart)
    (:Update
      (Utilities|Time|SetGlobalTimeDilation _newtrack_0))))

(event EventBeginPlay
  (Input|EnableInput (Game|GetPlayerController 0)))

(event Collision|EventActorBeginOverlap
  (params (OtherActor :type Actor%20Object%20Reference)))

(event EventTick
  (params (DeltaSeconds :type Float%20%28single-precision%29))
  (bind _returnvalue (Class|GameplayStatics|GetGlobalTimeDilation))
  (Development|PrintString (Utilities|String|Append "GTD: " (Utilities|String|ToString(Float) _returnvalue)) true true "(R=0.000000,G=0.660000,B=1.000000,A=1.000000)" _returnvalue)
  (if (Variables|Default|GetbeingLookedAt)
    (CallFunction|PlayerLookingat)))

(event Input|ActionEvents|InputActionScrewaround
  (params (Key :type Key%20Structure))
  (:Pressed
    (Variables|Default|SetbeingLookedAt true))
  (:Released
    (Variables|Default|SetbeingLookedAt false)
    (CallFunction|PlayerLookAway)))

(fn ConstructionScript)

(fn BeginSlowMo
  (params (Player :type Character%20Object%20Reference))
  (Development|PrintString "slowMoStart")
  (Utilities|Time|SetGlobalTimeDilation 0.5))

(fn BeginGrabSequence
  (Development|PrintString "grabStart")
  (Utilities|Time|SetGlobalTimeDilation 1.0))

(fn SlowMoEnd)

(fn SticktoClaws
  (bind _playerref (Variables|Default|GetPlayerRef))
  (Utilities|IsValid _playerref
    (:Is%20Valid
      (Transformation|AttachActorToActor _playerref "Claw" "KeepRelative" "KeepRelative" "KeepRelative" true)
      (Collision|SetCollisionEnabled (Variables|Default|GetgrabSphere) "NoCollision"))))

(fn PlayerLookingat
  (bind _returnvalue (Game|GetPlayerController 0))
  (bind _returnvalue_2 (Transformation|GetActorLocation))
  (bind _springarm (Variables|Default|GetSpringArm))
  (bind _returnvalue_3 (Pawn|GetControlledPawn _returnvalue))
  (bind _returnvalue_4 (Transformation|GetActorLocation _returnvalue_3))
  (Variables|/Script/Engine.SpringArmComponent|SetTargetArmLength _springarm (/ (Math|Vector|VectorLength (- _returnvalue_4 _returnvalue_2)) 2.0))
  (Transformation|SetWorldRotation _springarm (Math|Rotator|FindLookatRotation _returnvalue_4 _returnvalue_2) false false)
  (Game|Player|SetViewTargetwithBlend (Game|GetPlayerController 0) self 0.25 "VTBlend_Linear" 0.0 false))

(fn PlayerLookAway
  (bind _returnvalue (Game|GetPlayerController 0))
  (Game|Player|SetViewTargetwithBlend _returnvalue (Pawn|GetControlledPawn _returnvalue) 0.0 "VTBlend_Linear" 0.0 false))