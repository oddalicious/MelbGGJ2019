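; BP_StickGrabTarget is a stick grab target that varies its appearance at random.
; On BeginPlay, if StickOptions has entries, it checks a randomly indexed entry for validity and sets StaticMesh from a random index.
; The validity check and the mesh assignment each roll their own random index, so they can refer to different entries.
; The construction script only calls the parent's.
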(event EventBeginPlay
  (bind _stickoptions (Variables|Default|GetStickOptions))
  (bind _returnvalue (Utilities|Array|Length _stickoptions))
  (bind _returnvalue_2 (Math|Random|RandomInteger _returnvalue))
  (bind _output (Utilities|Array|Get(acopy) _stickoptions _returnvalue_2))
  (if (> _returnvalue 0)
    (Utilities|IsValid _output
      (:Is%20Valid
        (Components|StaticMesh|SetStaticMesh (Variables|Default|GetStaticMesh) _output)))))

(fn ConstructionScript
  (|CallParentFunction))