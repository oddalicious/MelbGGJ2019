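; BP_RabbitTarget is a rabbit character that acts as a grab target and can be caught by the player's claws.
; Begin and end target events toggle custom depth on the mesh.
; When stuck to the claws, it runs the parent behavior, turns off gravity, flags its ABP_Rabbit animation instance as dead, and destroys itself after a short delay.
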(event EventBeginTarget
  (Rendering|SetRenderCustomDepth (Variables|Character|GetMesh) true))

(event EventEndTarget
  (Rendering|SetRenderCustomDepth (Variables|Character|GetMesh) false))

(event EventSticktoClaws
  (params (Player%20Ref :type BP%20Player%20Object%20Reference))
  (|CallParentFunction Player%20Ref)
  (Variables|/Script/Engine.CharacterMovementComponent|SetGravityScale (Variables|Character|GetCharacterMovement) 0.0)
  (Physics|SetEnableGravity (Variables|Character|GetMesh) false)
  (bind _asabp_rabbit (Utilities|Casting|CastToABP_Rabbit (Components|SkeletalMesh|GetAnimInstance (Variables|Character|GetMesh))))
  (Variables|/Game/Blueprints/GrabTarget/Animal/ABP_Rabbit.ABP_Rabbit_C|SetisDead _asabp_rabbit true)
  (Utilities|FlowControl|Delay 3.0)
  (Actor|DestroyActor))

(fn ConstructionScript
  (|CallParentFunction))