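; Game mode that handles player death and respawn behind a screen fade.
; One timeline drives the fade widget's opacity: fading in destroys the pawn when finished, fading out plays it in reverse.
; The pawn's destroyed event triggers a delayed spawn and possession of a new BP_Player at SpawnTransform, then fades out and rebinds to the new pawn.
; Debug widget creation is present but unwired.
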(event Custom|PlayFadeIn
  (bind _direction (Timeline|DeathFadeInOut PlayFromStart)
    (:Update
      (Default|SetFadeOpacity (Variables|Default|GetFadeHUDRef) (Components|Timeline|GetPlaybackPosition (Variables|Default|GetDeathFadeInOut))))
    (:Finished
      (switch Utilities|FlowControl|Switch|SwitchonETimelineDirection _direction
        (:Forward
          (Actor|DestroyActor (Game|Player|GetPlayerPawn 0)))))))

(event Custom|PlayFadeOut
  (bind _direction (Timeline|DeathFadeInOut ReverseFromEnd)
    (:Update
      (Default|SetFadeOpacity (Variables|Default|GetFadeHUDRef) (Components|Timeline|GetPlaybackPosition (Variables|Default|GetDeathFadeInOut))))
    (:Finished
      (switch Utilities|FlowControl|Switch|SwitchonETimelineDirection _direction
        (:Forward
          (Actor|DestroyActor (Game|Player|GetPlayerPawn 0)))))))

(event Custom|Respawn
  (CallFunction|PlayFadeOut)
  (bind _asbp_player (Utilities|Casting|CastToBP_Player (Game|Player|GetPlayerPawn 0)))
  (Game|BindEventtoOnDestroyed _asbp_player (delegate Custom|OnPlayerDestroyedEvent)))

(event Custom|OnPlayerDestroyedEvent
  (params (DestroyedActor :type Actor%20Object%20Reference))
  (Utilities|FlowControl|Delay 1.0)
  (bind _returnvalue (Game|SpawnActorfromClass "/Game/Blueprints/BP_Player.BP_Player_C" (Variables|Default|GetSpawnTransform) "Undefined" 0 0))
  (Pawn|Possess (Game|GetPlayerController 0) _returnvalue)
  (CallFunction|Respawn))

(event EventBeginPlay
  (Utilities|FlowControl|Sequence
    (:then_0
      (Utilities|SetupLerpTimeline (Variables|Default|GetDeathFadeInOut) "/Game/Data/Curve_LinearLerp_Float.Curve_LinearLerp_Float" (Variables|Default|GetFadeSpeed) 1.0 false
        (:__
          (bind _asbp_player (Utilities|Casting|CastToBP_Player (Game|Player|GetPlayerPawn 0)))
          (Game|BindEventtoOnDestroyed _asbp_player (delegate Custom|OnPlayerDestroyedEvent)))))
    (:then_1
      (bind _returnvalue (UserInterface|CreateWidget "/Game/Blueprints/WBP_Fade.WBP_Fade_C"))
      (bind _output_get (Variables|Default|SetFadeHUDRef _returnvalue))
      (UserInterface|Viewport|AddtoViewport _output_get 0))))

(fn ConstructionScript)

(fn Fadein
  (CallFunction|PlayFadein))

(fn FadeOut
  (CallFunction|PlayFadeOut))